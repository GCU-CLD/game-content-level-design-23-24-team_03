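; MandatoryCollectible_BP is a pickup that the player collects by overlapping it.
; A timeline started on BeginPlay replays endlessly to animate the mesh's relative location and yaw, with pitch held fixed.
; When the first player's pawn overlaps it, the actor passes itself to ALS_GameMode_SP's CollectCollectible, plays a sound and destroys itself.
; If the game mode cast fails, the pickup stays in place.
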(event `self.ReceiveBeginPlay`
  (bind (_direction _location _rotation) (`Timeline|Timeline`)
    (:`Update`
      (`SceneComponent.K2_SetRelativeLocationAndRotation` (`self. Mesh`) _location (`KismetMathLibrary.MakeRotator` 0.0 90.0 (.z _rotation)) false false))
    (:`Finished`
      (`TimelineComponent.PlayFromStart` (`self.Timeline`)))))

(event `self.ReceiveActorBeginOverlap`
  (params (OtherActor :type "Actor Object Reference"))
  (if (== (`Controller.K2_GetPawn` (`GameplayStatics.GetPlayerController` 0)) OtherActor)
    (bind _asals_game_mode_sp (cast `/Game/AdvancedLocomotionV4/Blueprints/GameModes/ALS_GameMode_SP` (`GameplayStatics.GetGameMode`)))
    (`/Game/AdvancedLocomotionV4/Blueprints/GameModes/ALS_GameMode_SP.CollectCollectible` _asals_game_mode_sp self)
    (`GameplayStatics.PlaySoundAtLocation` "/Game/PGTemplate/Audio/Collect_Cue.Collect_Cue" (`self.K2_GetActorLocation`) (struct) 1.0 1.0 0.0 null null null null)
    (`self.K2_DestroyActor`)))

(fn `UserConstructionScript`)